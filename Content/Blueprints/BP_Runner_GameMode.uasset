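; Game mode for a runner game that builds the initial track of moving platforms when play begins.
; BeginPlay repeatedly calls SpawnPlatform, which spawns a MovingPlatform at NextSpawnPoint, then moves that point to the new platform's SpawnPoint location, chaining platforms end to end.
; SpawnPlatform2 does the same with MovingPlatform2 on the shared point, but is not called within this Blueprint.
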(event EventBeginPlay
  (for _index (range 0 10)
    (CallFunction|SpawnPlatform)))

(fn ConstructionScript)

(fn SpawnPlatform
  (bind _returnvalue (Game|SpawnActorfromClass "/Game/Blueprints/MovingPlatform.MovingPlatform_C" (Variables|Default|GetNext%20Spawn%20Point) "Undefined" 0 0))
  (bind _asmoving_platform (Utilities|Casting|CastToMovingPlatform _returnvalue))
  (Variables|Default|SetNext%20Spawn%20Point (Math|Transform|MakeTransform (Transformation|GetWorldLocation (Variables|/Game/Blueprints/MovingPlatform.MovingPlatform_C|GetSpawn%20Point _asmoving_platform)) "0, 0, 0" "1,1,1")))

(fn SpawnPlatform2
  (bind _returnvalue (Game|SpawnActorfromClass "/Game/Blueprints/MovingPlatform2.MovingPlatform2_C" (Variables|Default|GetNext%20Spawn%20Point) "Undefined" 0 0))
  (bind _asmoving_platform_2 (Utilities|Casting|CastToMovingPlatform2 _returnvalue))
  (Variables|Default|SetNext%20Spawn%20Point (Math|Transform|MakeTransform (Transformation|GetWorldLocation (Variables|/Game/Blueprints/MovingPlatform2.MovingPlatform2_C|GetSpawn%20Point _asmoving_platform_2)) "0, 0, 0" "1,1,1")))